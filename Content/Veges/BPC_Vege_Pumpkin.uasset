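; Growable pumpkin vegetable whose stem and fruit scale up over time until it is flagged as grown.
; BeginPlay attaches two collision-free, zero-scale static mesh components to Fruit_Socket on the skeletal mesh.
; Tick adds fixed, frame-rate-dependent steps, growing fruit alongside the stem and setting IsGrown once both reach full size.
; Player overlap with the skeletal mesh only prints whether it is grown.
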(event OnComponentBeginOverlap(SkeletalMesh)
  (params (OverlappedComponent :type Primitive%20Component%20Object%20Reference) (OtherActor :type Actor%20Object%20Reference) (OtherComp :type Primitive%20Component%20Object%20Reference) (OtherBodyIndex :type Integer) (bFromSweep :type Boolean) (SweepResult :type Hit%20Result%20Structure%20%28by%20ref%29))
  (Utilities|Casting|CastToBP_CPlayer OtherActor)
  (if (Variables|Default|GetisGrown)
    (Development|PrintString "IsGrown")
    (else
      (Development|PrintString "NoGrown"))))

(event EventBeginPlay
  (bind (_returnvalue _returnvalue1) (CallFunction|Spawn "Fruit_Socket")))

(event Collision|EventActorBeginOverlap
  (params (OtherActor :type Actor%20Object%20Reference)))

(event EventTick
  (params (DeltaSeconds :type Float%20%28single-precision%29))
  (Transformation|SetRelativeScale3D (Variables|Default|GetSkeletalMesh) (Math|Conversions|ToVector(Float) (Variables|Default|GetStempGrow)))
  (if (>= (Variables|Default|GetStempGrow) 1.0)
    (if (>= (Variables|Default|GetStempGrow) 0.5)
      (if (>= (Variables|Default|GetFruitGrow) 1.0)
        (Variables|Default|SetisGrown true)
        (else
          (Variables|Default|SetFruitGrow (+ (Variables|Default|GetFruitGrow) 0.001) :!label _label)
          (Transformation|SetRelativeScale3D (stale EventBeginPlay _returnvalue) (Math|Conversions|ToVector(Float) (Variables|Default|GetFruitGrow))))))
    (else
      (Variables|Default|SetStempGrow (+ (Variables|Default|GetStempGrow) 0.001))
      (goto _label))))

(fn ConstructionScript)

(fn Spawn
  (params (SocketName :type Name))
  (bind _skeletalmesh (Variables|Default|GetSkeletalMesh))
  (bind _returnvalue (AddComponent|AddStaticMeshComponent false))
  (bind _returnvalue_2 (AddComponent|AddStaticMeshComponent false))
  (Collision|SetCollisionEnabled _returnvalue_2 "NoCollision")
  (Transformation|AttachComponentToComponent _returnvalue _skeletalmesh SocketName "KeepRelative" "KeepRelative" "KeepRelative" true)
  (Transformation|AttachComponentToComponent _returnvalue_2 _skeletalmesh SocketName "KeepRelative" "KeepRelative" "KeepRelative" true)
  (Transformation|SetRelativeScale3D _returnvalue_2 "0, 0, 0")
  (return _returnvalue _returnvalue_2))