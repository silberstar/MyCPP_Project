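; Carrot vegetable Blueprint that grows over time and reports whether it is ripe.
; Tick raises FruitGrow by a fixed per-frame step until it reaches full, then sets IsGrown.
; When a BP_CPlayer overlaps the skeletal mesh, it prints the grown or not-grown state as debug text.
; Scaling by growth is never executed, and the Spawn function taking a socket name is an empty stub.
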(event OnComponentBeginOverlap(SkeletalMesh)
  (params (OverlappedComponent :type Primitive%20Component%20Object%20Reference) (OtherActor :type Actor%20Object%20Reference) (OtherComp :type Primitive%20Component%20Object%20Reference) (OtherBodyIndex :type Integer) (bFromSweep :type Boolean) (SweepResult :type Hit%20Result%20Structure%20%28by%20ref%29))
  (Utilities|Casting|CastToBP_CPlayer OtherActor)
  (if (Variables|Default|GetisGrown)
    (Development|PrintString "IsGrown")
    (else
      (Development|PrintString "NoGrown"))))

(event EventBeginPlay)

(event Collision|EventActorBeginOverlap
  (params (OtherActor :type Actor%20Object%20Reference)))

(event EventTick
  (params (DeltaSeconds :type Float%20%28single-precision%29))
  (if (>= (Variables|Default|GetFruitGrow) 1.0)
    (Variables|Default|SetisGrown true)
    (else
      (Variables|Default|SetFruitGrow (+ (Variables|Default|GetFruitGrow) 0.001)))))

(fn ConstructionScript)

(fn Spawn
  (params (SocketName :type Name)))